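; BP_FlipFlopBoomerang is a thrown flip-flop weapon that flies to a destination and returns to the player.
; BoomerangTo clears the character's equipped child actor and switches its idle position, then moves the actor out over the given time.
; After a short delay it moves back to the player's location as sampled then, rotating before each leg.
; It then flags completion, re-equips the flip-flop, restores the idle position and destroys itself.
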(event Custom|Boomerang%20To
  (params (Destination :type Vector) (Time :type Float%20%28double-precision%29))
  (bind _asbp_third_person_character (Utilities|Casting|CastToBP_ThirdPersonCharacter (Game|GetPlayerCharacter 0)))
  (ChildActorComponent|SetChildActorClass (Variables|/Game/ThirdPerson/Blueprints/BP_ThirdPersonCharacter.BP_ThirdPersonCharacter_C|GetEquipedWeapon _asbp_third_person_character) 0)
  (Variables|/Game/ThirdPerson/Blueprints/BP_ThirdPersonCharacter.BP_ThirdPersonCharacter_C|SetIdlePosition _asbp_third_person_character "NewEnumerator2")
  (Transformation|AddActorLocalRotation "0.000000,90.000000,0.000000" true false)
  (Components|MoveComponentTo (Variables|Default|GetDefaultSceneRoot) Destination "0, 0, 0" false false Time false)
  (Utilities|FlowControl|Delay 0.3)
  (bind _asbp_third_person_character_2 (Utilities|Casting|CastToBP_ThirdPersonCharacter (Game|GetPlayerCharacter 0)))
  (Transformation|AddActorLocalRotation "0.000000,90.000000,0.000000" true false)
  (Components|MoveComponentTo (Variables|Default|GetDefaultSceneRoot) (Transformation|GetActorLocation _asbp_third_person_character_2) "0, 0, 0" false false 0.2 false)
  (Variables|Default|SetHas%20Finished%20Boomerang true)
  (bind _asbp_third_person_character_3 (Utilities|Casting|CastToBP_ThirdPersonCharacter (Game|GetPlayerCharacter 0)))
  (ChildActorComponent|SetChildActorClass (Variables|/Game/ThirdPerson/Blueprints/BP_ThirdPersonCharacter.BP_ThirdPersonCharacter_C|GetEquipedWeapon _asbp_third_person_character_3) "BP_FlipFlopBoomerang_C")
  (Variables|/Game/ThirdPerson/Blueprints/BP_ThirdPersonCharacter.BP_ThirdPersonCharacter_C|SetIdlePosition _asbp_third_person_character_3 "NewEnumerator1")
  (Actor|DestroyActor))

(fn ConstructionScript
  (|CallParentFunction))